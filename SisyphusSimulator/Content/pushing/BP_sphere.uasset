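; BP_sphere is a pushable sphere that the third-person character moves while interacting with it.
; Overlap events toggle the character's CanInteract flag, without checking which actor overlapped.
; Each Tick, while IsInteracting and CanInteract are true, the character's movement axes feed Speed/Direction.
; That function interpolates the sphere's relative location along its right vector for forward/back or forward vector for right/left, without sweep.
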(event EventBeginPlay
  (bind _returnvalue (Actor|GetActorOfClass "/Game/ThirdPerson/Blueprints/BP_ThirdPersonCharacter.BP_ThirdPersonCharacter_C"))
  (Variables|Default|SetCharREF _returnvalue))

(event EventTick
  (params (DeltaSeconds :type Float%20%28single-precision%29))
  (bind _charref (Variables|Default|GetCharREF))
  (bind _charref_2 (Variables|Default|GetCharREF))
  (bind _forward_backwards_axis (Variables|/Game/ThirdPerson/Blueprints/BP_ThirdPersonCharacter.BP_ThirdPersonCharacter_C|GetForward%20Backwards%20Axis _charref_2))
  (bind _right_left_axis (Variables|/Game/ThirdPerson/Blueprints/BP_ThirdPersonCharacter.BP_ThirdPersonCharacter_C|Getright%20left%20axis _charref_2))
  (if (Variables|/Game/ThirdPerson/Blueprints/BP_ThirdPersonCharacter.BP_ThirdPersonCharacter_C|GetisInteracting _charref)
    (if (Variables|/Game/ThirdPerson/Blueprints/BP_ThirdPersonCharacter.BP_ThirdPersonCharacter_C|GetCanInteract _charref)
      (Utilities|FlowControl|Sequence
        (:then_0
          (if (== _forward_backwards_axis 0.0)
            (Development|PrintString "not moving forwards or bakcwards")
            (elif (>= _forward_backwards_axis 0.1)
              (Development|PrintString "is moving foraward")
              (Utilities|Speed/Direction true 34.0)
              (else
                (Development|PrintString "is moving backwards")
                (Utilities|Speed/Direction true -34.0)))))
        (:then_1
          (if (== _right_left_axis 0.0)
            (Development|PrintString "not moving forwards or bakcwards")
            (elif (>= _right_left_axis 0.1)
              (Development|PrintString "is moving right")
              (Utilities|Speed/Direction false -3e+01)
              (else
                (Development|PrintString "is moving left")
                (Utilities|Speed/Direction false 3e+01)))))))))

(event Collision|EventActorBeginOverlap
  (params (OtherActor :type Actor%20Object%20Reference))
  (Development|PrintString "interacting")
  (Variables|/Game/ThirdPerson/Blueprints/BP_ThirdPersonCharacter.BP_ThirdPersonCharacter_C|SetCanInteract (Variables|Default|GetCharREF) true))

(event Collision|EventActorEndOverlap
  (params (OtherActor :type Actor%20Object%20Reference))
  (Development|PrintString "NOT interacitng")
  (Variables|/Game/ThirdPerson/Blueprints/BP_ThirdPersonCharacter.BP_ThirdPersonCharacter_C|SetCanInteract (Variables|Default|GetCharREF) false))

(fn ConstructionScript)