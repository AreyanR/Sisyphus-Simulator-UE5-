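; Boulder Blueprint in the pushing folder, with a single graph that moves its sphere shape at a given speed and direction.
; Speed/Direction picks the sphere's right or forward vector from FwdBkwd, flips its X and Y, and scales up Z.
; It adds that offset to the relative location and eases toward it with VInterpTo at DirectionSpeed, setting the location without sweep collision.
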(fn ConstructionScript)