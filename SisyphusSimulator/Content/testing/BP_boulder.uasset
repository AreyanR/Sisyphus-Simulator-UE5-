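; Test boulder Actor meant to be pushed by the third-person character while that character is interacting and any actor overlap has enabled CanInteract.
; Tick reads the character's movement axes and calls Speed/Direction with a signed speed, printing a debug "Hello" on forward input.
; Speed/Direction uses VInterpTo on the sphere's relative location, but its direction vector is multiplied by zero, so the target equals the current position.
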(event EventBeginPlay
  (bind _returnvalue (Actor|GetActorOfClass "/Game/ThirdPerson/Blueprints/BP_ThirdPersonCharacter.BP_ThirdPersonCharacter_C"))
  (Variables|Default|SetChar _returnvalue))

(event EventTick
  (params (DeltaSeconds :type Float%20%28single-precision%29))
  (bind _char (Variables|Default|GetChar))
  (bind _char_2 (Variables|Default|GetChar))
  (bind _forward_backwards_axis (Variables|/Game/ThirdPerson/Blueprints/BP_ThirdPersonCharacter.BP_ThirdPersonCharacter_C|GetForward%20Backwards%20Axis _char_2))
  (bind _right_left_axis (Variables|/Game/ThirdPerson/Blueprints/BP_ThirdPersonCharacter.BP_ThirdPersonCharacter_C|Getright%20left%20axis _char_2))
  (if (Variables|/Game/ThirdPerson/Blueprints/BP_ThirdPersonCharacter.BP_ThirdPersonCharacter_C|GetisInteracting _char)
    (if (Variables|/Game/ThirdPerson/Blueprints/BP_ThirdPersonCharacter.BP_ThirdPersonCharacter_C|GetCanInteract _char)
      (Utilities|FlowControl|Sequence
        (:then_0
          (if (not (== _forward_backwards_axis 0.0))
            (if (>= _forward_backwards_axis 0.1)
              (Development|PrintString "Hello")
              (Utilities|Speed/Direction true 25.0)
              (else
                (Utilities|Speed/Direction true -25.0)))))
        (:then_1
          (if (not (== _right_left_axis 0.0))
            (if (>= _right_left_axis 0.1)
              (Utilities|Speed/Direction false -25.0)
              (else
                (Utilities|Speed/Direction false 25.0)))))))))

(event Collision|EventActorBeginOverlap
  (params (OtherActor :type Actor%20Object%20Reference))
  (Variables|/Game/ThirdPerson/Blueprints/BP_ThirdPersonCharacter.BP_ThirdPersonCharacter_C|SetCanInteract (Variables|Default|GetChar) true))

(event Collision|EventActorEndOverlap
  (params (OtherActor :type Actor%20Object%20Reference))
  (Variables|/Game/ThirdPerson/Blueprints/BP_ThirdPersonCharacter.BP_ThirdPersonCharacter_C|SetCanInteract (Variables|Default|GetChar) false))

(fn ConstructionScript)